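; Cuttable tree actor that gives the player logs when interacted with at close range.
; The CutDistance overlap sets a range flag and sends itself and a cut prompt to the overlapping actor; end overlap clears the flag but targets its message resets at OverlappedComponent.
; StartInteraction checks the flag, adds a clamped random log count to BP_PlayerCharacter, then swaps the tree mesh for a stump via visibility, without disabling further interaction.
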(event `/Game/UX/BPI_Interaction_Obj.Start Interaction`
  (params (Character :type "Character Object Reference"))
  (if (`self.DistanceTrue`)
    (bind _asthird_person_character (cast `/Game/ThirdPersonBP/Blueprints/BP_PlayerCharacter` Character))
    (`/Game/ThirdPersonBP/Blueprints/BP_PlayerCharacter.Add Log` _asthird_person_character (`KismetMathLibrary.Clamp` (`KismetMathLibrary.RandomInteger` 15) 1 10))
    (`SceneComponent.SetHiddenInGame` (`self.SM_tree_01`) true false)
    (`SceneComponent.SetHiddenInGame` (`self.SM_stump_01`) false false)))

(event `self.Cut Distance.OnComponentBeginOverlap`
  (params (OverlappedComponent :type "PrimitiveComponent Object Reference") (OtherActor :type "Actor Object Reference") (OtherComp :type "PrimitiveComponent Object Reference") (OtherBodyIndex :type Integer) (bFromSweep :type Boolean) (SweepResult :type "HitResult Structure (by ref)"))
  (set `self.DistanceTrue` true)
  (message `/Game/UX/BP_Interact.Set_Interactable_Object` OtherActor self)
  (bind _is_player_ (message `/Game/UX/BP_Interact.Player_Interact_Overlay` OtherActor))
  (if _is_player_
    (if (`self.DistanceTrue`)
      (message `/Game/UX/BP_Interact.Set_Interact_Text` OtherActor "Press E to Cut")
      (else
        (message `/Game/UX/BP_Interact.Set_Interact_Text` OtherActor "")))))

(event `self.Cut Distance.OnComponentEndOverlap`
  (params (OverlappedComponent :type "PrimitiveComponent Object Reference") (OtherActor :type "Actor Object Reference") (OtherComp :type "PrimitiveComponent Object Reference") (OtherBodyIndex :type Integer))
  (set `self.DistanceTrue` false)
  (message `/Game/UX/BP_Interact.Set_Interactable_Object` OverlappedComponent null)
  (message `/Game/UX/BP_Interact.Set_Interact_Text` OverlappedComponent ""))

(fn `UserConstructionScript`)