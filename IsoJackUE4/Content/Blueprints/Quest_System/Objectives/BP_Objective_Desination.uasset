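; BP_Objective_Desination is a quest objective step that completes when the player reaches a destination actor.
; On activation it binds to the Destination actor's begin-overlap event.
; When a BP_PlayerCharacter overlaps it, the step unbinds, sets ReachedDestination and fires the step-completed call.
; Its completion query simply returns that flag.
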(event `self.Activate_Objective_Step`
  (`parent.Activate_Objective_Step`)
  (add `Actor.OnActorBeginOverlap` (`self.Destination`) (delegate `OnActorBeginOverlap_Event_0`)))

(event `OnActorBeginOverlap_Event_0`
  (params (OverlappedActor :type "Actor Object Reference") (OtherActor :type "Actor Object Reference"))
  (cast `/Game/ThirdPersonBP/Blueprints/BP_PlayerCharacter` OtherActor)
  (remove `Actor.OnActorBeginOverlap` (`self.Destination`) (delegate `OnActorBeginOverlap_Event_0`))
  (set `self.Reached_Destination` true)
  (`self.On_step_Completed` self))

(fn `Get_Is_Completed`
  (returns (IsComplete :type Boolean))
  (return (`self.Reached_Destination`)))