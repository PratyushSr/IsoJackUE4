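; BP_Quest_Root is the base Blueprint for quests, which are built around a root objective collection.
; On BeginPlay it constructs and stores that collection, populates it with objectives, then activates its objective step.
; The construct and populate functions are placeholders that only print error messages, so child quests are expected to override them, while a getter exposes the stored collection.
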(event `self.ReceiveBeginPlay`
  (bind _rootobjectcollection (`self.Construct_root_Objective_Collection`))
  (bind _output_get (set `self.Root_Objective_Collection` _rootobjectcollection))
  (`self.Populate_Objectives` _output_get)
  (`/Game/Blueprints/Quest_System/Objectives/BP_Objective.Activate_Objective_Step` (`self.Root_Objective_Collection`)))

(fn `Construct_root_Objective_Collection`
  (returns (RootObjectCollection :type "/Game/Blueprints/Quest_System/Objectives/BP_Obj_Collection Object Reference"))
  (`KismetSystemLibrary.PrintString` "Error: CreateRootObjectiveCollection called for base class! Check :BP_Quest_Root:" true true (struct :`R` 1.0 :`A` 1.0) 5.0)
  (return null))

(fn `Get_Root_Objective_Collection`
  (returns (Root_Objective_Collection :type "/Game/Blueprints/Quest_System/Objectives/BP_Obj_Collection Object Reference"))
  (return (`self.Root_Objective_Collection`)))

(fn `Populate_Objectives`
  (params (RootObjCollection_Populate :type "/Game/Blueprints/Quest_System/Objectives/BP_Obj_Collection Object Reference"))
  (`KismetSystemLibrary.PrintString` "Quest Does not have Objectives Setup, Check BP_Quest_root_ populate objective for more information." true true (struct :`R` 1.0 :`G` 0.718554 :`B` 0.099455 :`A` 1.0)))

(fn `UserConstructionScript`)