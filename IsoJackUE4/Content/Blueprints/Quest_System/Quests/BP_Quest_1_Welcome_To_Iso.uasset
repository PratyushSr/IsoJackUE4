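; BP_Quest_1_Welcome_To_Iso defines the "Welcome To Iso" quest, which sends the player around to three locations.
; It constructs a root objective collection that requires sequential completion.
; It then adds destination steps for the Village Chief's House, Jack's House and the Forge, each tied to its own trigger reference.
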(fn `Construct_root_Objective_Collection`
  (returns (RootObjectCollection :type "/Game/Blueprints/Quest_System/Objectives/BP_Obj_Collection Object Reference"))
  (bind _returnvalue (`|GenericCreateObject` "/Game/Blueprints/Quest_System/Objectives/BP_Obj_Collection.BP_Obj_Collection_C" self true "Welcome To Iso"))
  (return _returnvalue))

(fn `Populate_Objectives`
  (params (RootObjCollection_Populate :type "/Game/Blueprints/Quest_System/Objectives/BP_Obj_Collection Object Reference"))
  (`|ExecutionSequence`
    (:`then_0`
      (bind _returnvalue (`|GenericCreateObject` "/Game/Blueprints/Quest_System/Objectives/BP_Objective_Desination.BP_Objective_Desination_C" self (`self.Chief_House_trigger`) "Head over to the Village Chief's House"))
      (`/Game/Blueprints/Quest_System/Objectives/BP_Obj_Collection.Add_Objective_step` (`local.RootObjCollection_Populate`) _returnvalue))
    (:`then_1`
      (bind _returnvalue_2 (`|GenericCreateObject` "/Game/Blueprints/Quest_System/Objectives/BP_Objective_Desination.BP_Objective_Desination_C" self (`self.Jack_House_Trigger`) "Head over to Jack's House"))
      (`/Game/Blueprints/Quest_System/Objectives/BP_Obj_Collection.Add_Objective_step` (`local.RootObjCollection_Populate`) _returnvalue_2))
    (:`then_2`
      (bind _returnvalue_3 (`|GenericCreateObject` "/Game/Blueprints/Quest_System/Objectives/BP_Objective_Desination.BP_Objective_Desination_C" self (`self.Forge_Trigger`) "Head over to the Forge"))
      (`/Game/Blueprints/Quest_System/Objectives/BP_Obj_Collection.Add_Objective_step` (`local.RootObjCollection_Populate`) _returnvalue_3))))

(fn `UserConstructionScript`
  (`parent.UserConstructionScript`))