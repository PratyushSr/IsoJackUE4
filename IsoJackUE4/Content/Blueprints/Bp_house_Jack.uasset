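; House actor Bp_house_Jack with an interactive wooden door that the player can open and close.
; Box overlap registers the actor as the character's interactable through message calls and shows an open or close prompt based on DoorState; leaving clears both.
; StartInteraction clears the prompt, then a FlipFlop with paired DoOnce nodes alternates timed MoveComponentTo moves, with a busy flag guarding against re-triggering.
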(event `/Game/UX/BPI_Interaction_Obj.Start Interaction`
  (params (Character :type "Character Object Reference"))
  (bind _sm_stylized_wood_door (`self.SM_Stylized_Wood_Door`))
  (message `/Game/UX/BP_Interact.Set_Interact_Text` Character "")
  (if (`self.Not Opening/closing`)
    (set `self.Not Opening/closing` false)
    (`/Engine/EditorBlueprintResources/StandardMacros.FlipFlop`
      (:`A`
        (`|ExecutionSequence`
          (:`then_0`
            (`/Engine/EditorBlueprintResources/StandardMacros.DoOnce` false :!label _label
              (:`Completed`
                (set `self.DoorState` false)
                (`KismetSystemLibrary.MoveComponentTo` _sm_stylized_wood_door (-70.0 70.0 0.0) (struct :`Yaw` 90.0) false false 2.0)
                (set `self.Not Opening/closing` true))))
          (:`then_1`
            (goto _label_2 :!via `Reset`))))
      (:`B`
        (`|ExecutionSequence`
          (:`then_0`
            (`/Engine/EditorBlueprintResources/StandardMacros.DoOnce` false :!label _label_2
              (:`Completed`
                (set `self.DoorState` true)
                (`KismetSystemLibrary.MoveComponentTo` _sm_stylized_wood_door (0.0 0.0 0.0) (struct) false false 2.0)
                (set `self.Not Opening/closing` true))))
          (:`then_1`
            (goto _label :!via `Reset`)))))))

(event `self.Box.OnComponentBeginOverlap`
  (params (OverlappedComponent :type "PrimitiveComponent Object Reference") (OtherActor :type "Actor Object Reference") (OtherComp :type "PrimitiveComponent Object Reference") (OtherBodyIndex :type Integer) (bFromSweep :type Boolean) (SweepResult :type "HitResult Structure (by ref)"))
  (message `/Game/UX/BP_Interact.Set_Interactable_Object` OtherActor self)
  (bind _is_player_ (message `/Game/UX/BP_Interact.Player_Interact_Overlay` OtherActor))
  (if _is_player_
    (if (`self.DoorState`)
      (message `/Game/UX/BP_Interact.Set_Interact_Text` OtherActor "Press E to Open")
      (else
        (message `/Game/UX/BP_Interact.Set_Interact_Text` OtherActor "Press E to Close")))))

(event `self.Box.OnComponentEndOverlap`
  (params (OverlappedComponent :type "PrimitiveComponent Object Reference") (OtherActor :type "Actor Object Reference") (OtherComp :type "PrimitiveComponent Object Reference") (OtherBodyIndex :type Integer))
  (message `/Game/UX/BP_Interact.Set_Interactable_Object` OtherActor null)
  (message `/Game/UX/BP_Interact.Set_Interact_Text` OtherActor ""))

(fn `UserConstructionScript`)