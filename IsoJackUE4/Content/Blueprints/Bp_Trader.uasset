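; Trader actor that the player can interact with to start trading.
; Entering its box registers it as the overlapping actor's interactable through interface messages and, if that actor's overlay check passes, shows an "E" trade prompt.
; Leaving the box clears the interactable and prompt.
; StartInteraction looks up the ThirdPersonCharacter by class and calls BeginTrading on it, so the trader holds no trade logic itself.
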(event `/Game/UX/BPI_Interaction_Obj.Start Interaction`
  (params (Character :type "Character Object Reference"))
  (bind _returnvalue (`GameplayStatics.GetActorOfClass` "/Game/ThirdPersonBP/Blueprints/ThirdPersonCharacter.ThirdPersonCharacter_C"))
  (`/Game/ThirdPersonBP/Blueprints/ThirdPersonCharacter.Begin Trading` _returnvalue))

(event `self.Box.OnComponentBeginOverlap`
  (params (OverlappedComponent :type "PrimitiveComponent Object Reference") (OtherActor :type "Actor Object Reference") (OtherComp :type "PrimitiveComponent Object Reference") (OtherBodyIndex :type Integer) (bFromSweep :type Boolean) (SweepResult :type "HitResult Structure (by ref)"))
  (message `/Game/UX/BP_Interact.Set_Interactable_Object` OtherActor self)
  (bind _is_player_ (message `/Game/UX/BP_Interact.Player_Interact_Overlay` OtherActor))
  (if _is_player_
    (message `/Game/UX/BP_Interact.Set_Interact_Text` OtherActor "Press E to Trade")))

(event `self.Box.OnComponentEndOverlap`
  (params (OverlappedComponent :type "PrimitiveComponent Object Reference") (OtherActor :type "Actor Object Reference") (OtherComp :type "PrimitiveComponent Object Reference") (OtherBodyIndex :type Integer))
  (message `/Game/UX/BP_Interact.Set_Interactable_Object` OtherActor null)
  (message `/Game/UX/BP_Interact.Set_Interact_Text` OtherActor ""))

(fn `UserConstructionScript`)