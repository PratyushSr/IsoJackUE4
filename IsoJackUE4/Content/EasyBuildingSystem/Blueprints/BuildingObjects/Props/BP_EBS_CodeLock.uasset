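; Code lock building prop for the Easy Building System that players use with E to set a password or authorize.
; Use messages the pawn's PlayerState; CreateLockWidget opens the code lock UI with the player's authorization status and switches to UI-only input.
; A multicast event swaps the emissive texture between red (locked) and green (unlocked) through a dynamic material instance.
; The use prompt depends on lock state and player authorization.
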(event `/Game/EasyBuildingSystem/Blueprints/Interfaces/BPI_EBS_Usable.Use`
  (params (Pawn :type "Pawn Object Reference") (Key :type "Key Structure"))
  ;[1 1 1] Create Code Lock Widget.
  (if (== Key "E")
    (message `/Game/EasyBuildingSystem/Blueprints/Interfaces/BPI_EBS_MultiplayerEvents.CreateCodeLockWidget_BPI` (`Pawn.PlayerState` Pawn) self Pawn)
    (else
      (`parent.Use` Pawn Key))))

(event `CreateLockWidget`
  (params (Pawn :type "Pawn Object Reference"))
  (bind _asplayer_controller (cast `PlayerController` (`Pawn.GetController` Pawn) :!pure true))
  ;[1 1 1] Create Code Lock Widget.
  (bind _autorized (`self.CheckAutorizedPlayer` Pawn))
  (bind _returnvalue (`|CreateWidget` "/Game/EasyBuildingSystem/Blueprints/UserInterface/UI_EBS_CodeLock.UI_EBS_CodeLock_C" _asplayer_controller _autorized self))
  (`UserWidget.AddToViewport` _returnvalue 0)
  (`WidgetBlueprintLibrary.SetInputMode_UIOnlyEx` _asplayer_controller _returnvalue)
  (set `PlayerController.bShowMouseCursor` true _asplayer_controller))

(event `self.UpdateLockCosmetics (Multicast)`
  (bind _mesh (`self.Mesh`))
  (bind _returnvalue (`PrimitiveComponent.GetMaterial` _mesh 0))
  ;[1 1 1] Create Code Lock Widget.
  (if (not (`self.IsLocked`))
    (bind _returnvalue_2 (`PrimitiveComponent.CreateDynamicMaterialInstance` _mesh 0 _returnvalue))
    (`MaterialInstanceDynamic.SetTextureParameterValue` _returnvalue_2 "Emissive" "/Game/EasyBuildingSystem/Textures/Structures/T_CodeLock_001_E_Green.T_CodeLock_001_E_Green")
    (else
      (bind _returnvalue_3 (`PrimitiveComponent.CreateDynamicMaterialInstance` _mesh 0 _returnvalue))
      (`MaterialInstanceDynamic.SetTextureParameterValue` _returnvalue_3 "Emissive" "/Game/EasyBuildingSystem/Textures/Structures/T_CodeLock_001_E_Red.T_CodeLock_001_E_Red"))))

(fn `GetUsableText`
  (params (Pawn :type "Pawn Object Reference"))
  (returns (Text :type Text))
  (if (`self.IsLocked`)
    (bind _autorized (`self.CheckAutorizedPlayer` Pawn))
    (if _autorized
      (return "[E] Set password.")
      (else
        (return "[E] Autorize.")))
    (else
      (return "[E] Set password."))))

(fn `UserConstructionScript`
  (`parent.UserConstructionScript`))