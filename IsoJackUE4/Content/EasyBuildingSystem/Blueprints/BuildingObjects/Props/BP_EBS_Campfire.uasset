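; Placeable campfire prop for the Easy Building System that players can ignite or put out with E.
; It supplies four floor checkers and a build collision component for placement checks, which is destroyed through the DestroyBuildComponents override.
; Using it toggles the Burn flag and multicasts the fire particle state, while the prompt text follows that flag.
; The construction script sets particle auto-activation from Burn.
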(event `self.SetFloorCheckers`
  ;[1 1 1] Overrided Events.
  (set `self.FloorCheckers` (`|MakeArray` (`self.FloorChecker1`) (`self.FloorChecker2`) (`self.FloorChecker3`) (`self.FloorChecker4`))))

(event `self.DestroyBuildComponents`
  ;[1 1 1] Overrided Events.
  (`ActorComponent.K2_DestroyComponent` (`self.BuildCollision`)))

(event `/Game/EasyBuildingSystem/Blueprints/Interfaces/BPI_EBS_Usable.Use`
  (params (Pawn :type "Pawn Object Reference") (Key :type "Key Structure"))
  ;[1 1 1] Ignite campfire.
  (if (== Key "E")
    (`self.Ignite`)
    (else
      (`parent.Use` null "AnyKey"))))

(event `Ignite`
  ;[1 1 1] Ignite campfire.
  (set `self.Burn` (not (`self.Burn`)))
  (`self.UpdateFireParticles (Multicast)`))

(event `UpdateFireParticles (Multicast)`
  (bind _fireparticles (`self.FireParticles`))
  ;[1 1 1] Ignite campfire.
  (if (`self.Burn`)
    (`ActorComponent.Activate` _fireparticles false)
    (else
      (`ActorComponent.Deactivate` _fireparticles))))

(fn `CheckBuildCollisions`
  (params (Actor :type "Actor Object Reference"))
  (returns (NotBlocked :type Boolean))
  (return (`self.CheckActorCollisions` Actor (`self.BuildCollision`))))

(fn `GetUsableText`
  (params (Pawn :type "Pawn Object Reference"))
  (returns (Text :type Text))
  (if (`self.Burn`)
    (return "[E] Put out.")
    (else
      (return "[E] Ignite."))))

(fn `UserConstructionScript`
  (`parent.UserConstructionScript`)
  (`ActorComponent.SetAutoActivate` (`self.FireParticles`) (`self.Burn`)))