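; Placeable torch prop for the Easy Building System that players can ignite or put out with E.
; Using it toggles the Burn flag and multicasts the fire particle update to clients, while other keys fall through to the parent.
; The construction script sets particle auto-activation from Burn, and the usable prompt text follows the same flag.
; It supplies four collision checkers to the inherited prop system.
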(event `self.SetCheckers`
  ;[1 1 1] Overrided Events.
  (set `self.PropCheckers` (`|MakeArray` (`self.CheckPropCollision`) (`self.CheckPropCollision2`) (`self.CheckPropCollision3`) (`self.CheckPropCollision4`))))

(event `/Game/EasyBuildingSystem/Blueprints/Interfaces/BPI_EBS_Usable.Use`
  (params (Pawn :type "Pawn Object Reference") (Key :type "Key Structure"))
  ;[1 1 1] Ignite campfire.
  (if (== Key "E")
    (`self.Ignite`)
    (else
      (`parent.Use` null "AnyKey"))))

(event `Ignite`
  ;[1 1 1] Ignite campfire.
  (set `self.Burn` (not (`self.Burn`)))
  (`self.UpdateFireParticles (Multicast)`))

(event `UpdateFireParticles (Multicast)`
  (bind _fireparticles (`self.FireParticles`))
  ;[1 1 1] Ignite campfire.
  (if (`self.Burn`)
    (`ActorComponent.Activate` _fireparticles false)
    (else
      (`ActorComponent.Deactivate` _fireparticles))))

(fn `GetUsableText`
  (params (Pawn :type "Pawn Object Reference"))
  (returns (Text :type Text))
  (if (`self.Burn`)
    (return "[E] Put out.")
    (else
      (return "[E] Ignite."))))

(fn `UserConstructionScript`
  (`parent.UserConstructionScript`)
  (`ActorComponent.SetAutoActivate` (`self.FireParticles`) (`self.Burn`)))