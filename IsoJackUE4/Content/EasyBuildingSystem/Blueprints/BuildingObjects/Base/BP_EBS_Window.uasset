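; Window building piece for the Easy Building System that can only be placed into a window frame.
; It snaps to the frame's WindowSocket, and its build check passes only while that frame holds no valid window.
; On attach it teleports and attaches to the socket, and the window and frame store references to each other.
; Save and load extend the parent's logic by recording the frame's save ID, then re-attaching on load.
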(event `self.CheckAndAttachToTarget`
  (params (TargetObject :type "/Game/EasyBuildingSystem/Blueprints/BuildingObjects/Base/BP_EBS_BuildingObject Object Reference"))
  (bind _asbp_ebs_window_frame (cast `/Game/EasyBuildingSystem/Blueprints/BuildingObjects/Base/BP_EBS_WindowFrame` TargetObject))
  (set `/Game/EasyBuildingSystem/Blueprints/BuildingObjects/Base/BP_EBS_WindowFrame.WindowReference` self _asbp_ebs_window_frame)
  (set `self.WindowFrameReference` _asbp_ebs_window_frame)
  (bind _windowsocket (`/Game/EasyBuildingSystem/Blueprints/BuildingObjects/Base/BP_EBS_WindowFrame.WindowSocket` _asbp_ebs_window_frame))
  (`self.K2_SetActorTransform` (`SceneComponent.K2_GetComponentToWorld` _windowsocket) false true)
  (`self.K2_AttachToComponent` _windowsocket "None" "SnapToTarget" "SnapToTarget" "SnapToTarget"))

(fn `CheckBuildStatus`
  (params (TargetObject :type "/Game/EasyBuildingSystem/Blueprints/BuildingObjects/Base/BP_EBS_BuildingObject Object Reference"))
  (returns (CanBuild :type Boolean))
  (return (not (`KismetSystemLibrary.IsValid` (`/Game/EasyBuildingSystem/Blueprints/BuildingObjects/Base/BP_EBS_WindowFrame.WindowReference` (cast `/Game/EasyBuildingSystem/Blueprints/BuildingObjects/Base/BP_EBS_WindowFrame` TargetObject :!pure true))))))

(fn `CheckSnap`
  (params (TargetObject :type "/Game/EasyBuildingSystem/Blueprints/BuildingObjects/Base/BP_EBS_BuildingObject Object Reference"))
  (returns (Snap :type Boolean))
  (return (`|EnumEquality` (`/Game/EasyBuildingSystem/Blueprints/BuildingObjects/Base/BP_EBS_BuildingObject.BuildingType` TargetObject) "NewEnumerator5")))

(fn `LoadData_BPI`
  (params (SaveData :type "SaveGame Object Reference"))
  (returns (Success :type Boolean))
  (bind _asbp_ebs_game_save (cast `/Game/EasyBuildingSystem/Blueprints/Game/SaveData/BP_EBS_GameSave` SaveData :!pure true))
  (bind _success (`parent.LoadData_BPI` SaveData))
  (if _success
    (`self.CheckAndAttachToTarget` (cast `/Game/EasyBuildingSystem/Blueprints/BuildingObjects/Base/BP_EBS_BuildingObject` (`BlueprintMapLibrary.Map_Find` (`/Game/EasyBuildingSystem/Blueprints/Game/SaveData/BP_EBS_GameSave.SavedObjects` _asbp_ebs_game_save) (`.WindowFrameReferenceSaveID_5_9F923F134F50517FFFA0AA9B1EAD8891` (break `/Game/EasyBuildingSystem/Blueprints/Game/SaveData/STR_EBS_WindowData` (`BlueprintMapLibrary.Map_Find` (`/Game/EasyBuildingSystem/Blueprints/Game/SaveData/BP_EBS_GameSave.SavedWindowsData` _asbp_ebs_game_save) (`self.SaveID`))))) :!pure true))
    (return true)
    (else
      (return false))))

(fn `SaveData_BPI`
  (params (SaveData :type "SaveGame Object Reference"))
  (returns (Success :type Boolean))
  (bind _success (`parent.SaveData_BPI` SaveData))
  (if _success
    (`BlueprintMapLibrary.Map_Add` (`/Game/EasyBuildingSystem/Blueprints/Game/SaveData/BP_EBS_GameSave.SavedWindowsData` (cast `/Game/EasyBuildingSystem/Blueprints/Game/SaveData/BP_EBS_GameSave` SaveData :!pure true)) (`self.SaveID`) (make `/Game/EasyBuildingSystem/Blueprints/Game/SaveData/STR_EBS_WindowData` (`/Game/EasyBuildingSystem/Blueprints/BuildingObjects/Base/BP_EBS_BuildingObject.SaveID` (`self.WindowFrameReference`))))
    (return true)
    (else
      (return false))))

(fn `SnapToTarget`
  (params (TargetObject :type "/Game/EasyBuildingSystem/Blueprints/BuildingObjects/Base/BP_EBS_BuildingObject Object Reference") (InputRotation :type "Float (double-precision)") (HitLocation :type "Vector Structure") (GridMode :type Boolean) (SnappingMode :type Boolean))
  (returns (NewLocation :type "Vector Structure") (NewRotation :type "Rotator Structure"))
  (bind (_returnvalue_location _returnvalue_rotation) (`KismetMathLibrary.BreakTransform` (`SceneComponent.K2_GetComponentToWorld` (`/Game/EasyBuildingSystem/Blueprints/BuildingObjects/Base/BP_EBS_WindowFrame.WindowSocket` (cast `/Game/EasyBuildingSystem/Blueprints/BuildingObjects/Base/BP_EBS_WindowFrame` TargetObject :!pure true)))))
  (return _returnvalue_location _returnvalue_rotation))

(fn `UserConstructionScript`
  (`parent.UserConstructionScript`))