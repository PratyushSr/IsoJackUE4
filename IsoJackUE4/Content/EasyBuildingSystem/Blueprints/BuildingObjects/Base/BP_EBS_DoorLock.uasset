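; Buildable door lock for the Easy Building System that snaps to a door's socket, one per door, and registers itself on it.
; Pressing E locks it with a placeholder password, recording the player's name as authorized, and only listed names can unlock it.
; A multicast swaps the emissive texture between red and green to show lock state.
; Save/load overrides persist lock data and reattach it through the door's save ID.
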(event `self.Use`
  (params (Pawn :type "Pawn Object Reference") (Key :type "Key Structure"))
  (bind _playername (`self.GetPlayerName` Pawn))
  ;[1 1 1] Try lock or unlock door.
  (if (== Key "E")
    (if (`self.IsLocked`)
      (bind _autorized (`self.CheckAutorizedPlayer` Pawn))
      (if _autorized
        (`self.SetPassword` "" _playername))
      (else
        (`self.SetPassword` "Lock" _playername)))
    (else
      (`parent.Use` Pawn Key))))

(event `Autorize`
  (params (PlayerName :type String))
  ;[1 1 1] Try lock or unlock door.
  (`KismetArrayLibrary.Array_AddUnique` (`self.AutorizedPlayers`) PlayerName))

(event `SetPassword`
  (params (Password :type Text) (PlayerName :type String))
  ;[1 1 1] Try lock or unlock door.
  (bind _output_get (set `self.Password` Password))
  (`KismetArrayLibrary.Array_Clear` (`self.AutorizedPlayers`))
  (if (`KismetTextLibrary.NotEqual_TextText` _output_get "")
    (`KismetArrayLibrary.Array_AddUnique` (`self.AutorizedPlayers`) PlayerName)
    (set `self.IsLocked` true)
    (else
      (set `self.IsLocked` false)))
  (`self.UpdateLockCosmetics (Multicast)`))

(event `UpdateLockCosmetics (Multicast)`
  (bind _mesh (`self.Mesh`))
  (bind _returnvalue (`PrimitiveComponent.GetMaterial` _mesh 0))
  ;[1 1 1] Try lock or unlock door.
  (if (not (`self.IsLocked`))
    (bind _returnvalue_2 (`PrimitiveComponent.CreateDynamicMaterialInstance` _mesh 0 _returnvalue))
    (`MaterialInstanceDynamic.SetTextureParameterValue` _returnvalue_2 "Emissive" "/Game/EasyBuildingSystem/Textures/Structures/T_CodeLock_003_E_Green.T_CodeLock_003_E_Green")
    (else
      (bind _returnvalue_3 (`PrimitiveComponent.CreateDynamicMaterialInstance` _mesh 0 _returnvalue))
      (`MaterialInstanceDynamic.SetTextureParameterValue` _returnvalue_3 "Emissive" "/Game/EasyBuildingSystem/Textures/Structures/T_CodeLock_003_E_Red.T_CodeLock_003_E_Red"))))

(event `self.CheckAndAttachToTarget`
  (params (TargetObject :type "/Game/EasyBuildingSystem/Blueprints/BuildingObjects/Base/BP_EBS_BuildingObject Object Reference"))
  ;[1 1 1] Overrided Events.
  (bind _asbp_ebs_door (cast `/Game/EasyBuildingSystem/Blueprints/BuildingObjects/Base/BP_EBS_Door` TargetObject))
  (set `/Game/EasyBuildingSystem/Blueprints/BuildingObjects/Base/BP_EBS_Door.DoorLockReference` self _asbp_ebs_door)
  (set `self.DoorReference` _asbp_ebs_door)
  (`self.K2_AttachToComponent` (`/Game/EasyBuildingSystem/Blueprints/BuildingObjects/Base/BP_EBS_BuildingObject.Mesh` _asbp_ebs_door) "DoorLock" "SnapToTarget" "SnapToTarget" "SnapToTarget"))

(fn `CheckAutorizedPlayer`
  (params (Pawn :type "Pawn Object Reference"))
  (returns (Autorized :type Boolean))
  ;[1 1 1] Return true if pawns player is autorized player.
  (return (`KismetArrayLibrary.Array_Contains` (`self.AutorizedPlayers`) (`PlayerState.GetPlayerName` (`Pawn.PlayerState` Pawn)))))

(fn `CheckBuildStatus`
  (params (TargetObject :type "/Game/EasyBuildingSystem/Blueprints/BuildingObjects/Base/BP_EBS_BuildingObject Object Reference"))
  (returns (CanBuild :type Boolean))
  (return (not (`KismetSystemLibrary.IsValid` (`/Game/EasyBuildingSystem/Blueprints/BuildingObjects/Base/BP_EBS_Door.DoorLockReference` (cast `/Game/EasyBuildingSystem/Blueprints/BuildingObjects/Base/BP_EBS_Door` TargetObject :!pure true))))))

(fn `CheckSnap`
  (params (TargetObject :type "/Game/EasyBuildingSystem/Blueprints/BuildingObjects/Base/BP_EBS_BuildingObject Object Reference"))
  (returns (Snap :type Boolean))
  (return (`|EnumEquality` (`/Game/EasyBuildingSystem/Blueprints/BuildingObjects/Base/BP_EBS_BuildingObject.BuildingType` TargetObject) "NewEnumerator8")))

(fn `GetPlayerName`
  (params (Pawn :type "Pawn Object Reference"))
  (returns (PlayerName :type String))
  ;[1 1 1] Get player name from PlayerState.
  (return (`PlayerState.GetPlayerName` (`Controller.PlayerState` (`Pawn.GetController` Pawn)))))

(fn `GetUsableText`
  (params (Pawn :type "Pawn Object Reference"))
  (returns (Text :type Text))
  (if (`self.IsLocked`)
    (bind _autorized (`self.CheckAutorizedPlayer` Pawn))
    (if _autorized
      (return "[E] Unlock.")
      (else
        (return "Locked by another player.")))
    (else
      (return "[E] Lock."))))

(fn `LoadData_BPI`
  (params (SaveData :type "SaveGame Object Reference"))
  (returns (Success :type Boolean))
  (bind _asbp_ebs_game_save (cast `/Game/EasyBuildingSystem/Blueprints/Game/SaveData/BP_EBS_GameSave` SaveData :!pure true))
  (bind (_doorreferencesaveid _islocked _password _maxpasswordlenght _autorizedplayers) (break `/Game/EasyBuildingSystem/Blueprints/Game/SaveData/STR_EBS_DoorLockData` (`BlueprintMapLibrary.Map_Find` (`/Game/EasyBuildingSystem/Blueprints/Game/SaveData/BP_EBS_GameSave.SavedDoorLocksData` _asbp_ebs_game_save) (`self.SaveID`))))
  (bind _success (`parent.LoadData_BPI` SaveData))
  (if _success
    (`self.CheckAndAttachToTarget` (cast `/Game/EasyBuildingSystem/Blueprints/BuildingObjects/Base/BP_EBS_BuildingObject` (`BlueprintMapLibrary.Map_Find` (`/Game/EasyBuildingSystem/Blueprints/Game/SaveData/BP_EBS_GameSave.SavedObjects` _asbp_ebs_game_save) _doorreferencesaveid) :!pure true))
    (set `self.IsLocked` _islocked)
    (set `self.Password` _password)
    (set `self.MaxPasswordLength` _maxpasswordlenght)
    (set `self.AutorizedPlayers` _autorizedplayers)
    (`self.UpdateLockCosmetics (Multicast)`)
    (return true)
    (else
      (return false))))

(fn `SaveData_BPI`
  (params (SaveData :type "SaveGame Object Reference"))
  (returns (Success :type Boolean))
  (bind _success (`parent.SaveData_BPI` SaveData))
  (if _success
    (`BlueprintMapLibrary.Map_Add` (`/Game/EasyBuildingSystem/Blueprints/Game/SaveData/BP_EBS_GameSave.SavedDoorLocksData` (cast `/Game/EasyBuildingSystem/Blueprints/Game/SaveData/BP_EBS_GameSave` SaveData :!pure true)) (`self.SaveID`) (make `/Game/EasyBuildingSystem/Blueprints/Game/SaveData/STR_EBS_DoorLockData` (`/Game/EasyBuildingSystem/Blueprints/BuildingObjects/Base/BP_EBS_BuildingObject.SaveID` (`self.DoorReference`)) (`self.IsLocked`) (`self.Password`) (`self.MaxPasswordLength`) (`self.AutorizedPlayers`)))
    (return true)
    (else
      (return false))))

(fn `SnapToTarget`
  (params (TargetObject :type "/Game/EasyBuildingSystem/Blueprints/BuildingObjects/Base/BP_EBS_BuildingObject Object Reference") (InputRotation :type "Float (double-precision)") (HitLocation :type "Vector Structure") (GridMode :type Boolean) (SnappingMode :type Boolean))
  (returns (NewLocation :type "Vector Structure") (NewRotation :type "Rotator Structure"))
  (bind _mesh (`/Game/EasyBuildingSystem/Blueprints/BuildingObjects/Base/BP_EBS_BuildingObject.Mesh` TargetObject))
  (bind _socketname (`self.SocketName`))
  (return (`SceneComponent.GetSocketLocation` _mesh _socketname) (`SceneComponent.GetSocketRotation` _mesh _socketname)))

(fn `UserConstructionScript`
  (`parent.UserConstructionScript`))