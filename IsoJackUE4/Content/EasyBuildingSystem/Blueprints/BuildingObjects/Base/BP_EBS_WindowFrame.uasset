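; BP_EBS_WindowFrame is the window frame building object in the Easy Building System, holding a reference to an attached window.
; It overrides RemoveAttachedObject so that, when the window reference is valid, the removal cascades to that window before destroying its actor.
; If the Destruct flag is set, it first calls DestructMulticast with the window's destructible mesh and world transform.
; The construction script only calls the parent's.
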(event `self.RemoveAttachedObject`
  (params (Destruct :type Boolean))
  (bind _windowreference (`self.WindowReference`))
  ;[1 1 1] Overrided Events.
  (`/Engine/EditorBlueprintResources/StandardMacros.IsValid` _windowreference
    (:`Is Valid`
      (if Destruct
        (`self.Destruct (Multicast)` (`.DestructibleMesh_8_C79245184590E438671E3E86006ABCDA` (break `/Game/EasyBuildingSystem/Blueprints/BuildingObjects/STR_EBS_BuildingObjectSettings` (`/Game/EasyBuildingSystem/Blueprints/BuildingObjects/Base/BP_EBS_BuildingObject.Settings` _windowreference))) (`SceneComponent.K2_GetComponentToWorld` (`/Game/EasyBuildingSystem/Blueprints/BuildingObjects/Base/BP_EBS_BuildingObject.Mesh` _windowreference))))
      (`self.RemoveAttachedObject` _windowreference Destruct)
      (`self.K2_DestroyActor` _windowreference))))

(fn `UserConstructionScript`
  (`parent.UserConstructionScript`))