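; Base building object for props placed on floors or landscape in the Easy Building System.
; Snapping takes the target floor's height, optionally rounds XY to a grid, and applies yaw.
; Building requires each floor checker, set up by an overridable construction hook, to overlap an allowed surface, and every overlapping actor to pass collision checks.
; Editor-built instances snap Z to their target floor, attach and resolve their main build target.
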(event `self.CheckBuildInEditor`
  (bind (_main _outsnaplevel) (`self.GetMainBuildTarget` 0))
  (bind _returnvalue (`self.GetTransform`))
  (bind _buildtarget (`self.BuildTarget`))
  (bind _tags (`self.Tags`))
  ;[1 1 1] Overrided Events
  (if (`self.BuildedInEditor`)
    (`|ExecutionSequence`
      (:`then_0`
        (if (or (== (`self.BuildTarget`) self) (== (`/Game/EasyBuildingSystem/Blueprints/BuildingObjects/Base/BP_EBS_BuildingObject.BuildTarget` (`self.BuildTarget`)) self))
          (set `self.BuildTarget` null)
          (set `self.MainBuildTarget` self))
        (`KismetArrayLibrary.Array_AddUnique` _tags "ConstructInEditor")
        (`/Engine/EditorBlueprintResources/StandardMacros.IsValid` _buildtarget
          (:`Is Valid`
            (bind _snap (`self.CheckSnap` _buildtarget))
            (if _snap
              (`self.K2_SetActorTransform` (`KismetMathLibrary.MakeTransform` (`KismetMathLibrary.MakeVector` (.x (.location _returnvalue)) (.y (.location _returnvalue)) (`self.GetFloorZ` _buildtarget)) (.rotation _returnvalue) (.scale _returnvalue)) false true)
              (`self.CheckAndAttachToTarget` _buildtarget)
              (set `self.MainBuildTarget` _main)
              (set `self.BuildSnapLevel` _outsnaplevel)
              (else
                (set `self.BuildTarget` null)
                (set `self.MainBuildTarget` self :!label _label))))
          (:`Is Not Valid`
            (goto _label))))
      (:`then_1`
        (`self.SetFloorByTargetObject` (`self.BuildTarget`))))
    (else
      (`KismetArrayLibrary.Array_RemoveItem` _tags "ConstructInEditor"))))

(fn `CheckBuildStatus`
  (params (TargetObject :type "/Game/EasyBuildingSystem/Blueprints/BuildingObjects/Base/BP_EBS_BuildingObject Object Reference"))
  (returns (CanBuild :type Boolean))
  (locals (LocalCount :type Integer))
  (bind _overlappingactors (`self.GetOverlappingActors` self null))
  ;[1 1 1] Check Floor Object can be build.
  (bind _hasprop (`self.CheckProp`))
  (if _hasprop
    (set `local.LocalCount` (`KismetArrayLibrary.Array_Length` _overlappingactors))
    (for _array_element _overlappingactors
      (if (`self.CheckBuildCollisions` _array_element)
        (`/Engine/EditorBlueprintResources/StandardMacros.DecrementInt` (`local.LocalCount`))))
    (if (== (`local.LocalCount`) 0)
      (return true)
      (else
        _)))
  (return false))

(fn `CheckProp`
  (returns (HasProp :type Boolean))
  (locals (LocalFloorCheck :type Boolean))
  (bind _placedonlandscape (`self.PlacedOnLandscape`))
  (set `local.LocalFloorCheck` true)
  (for _array_element (`self.FloorCheckers`)
    (if (and _placedonlandscape (`self.PlacedOnFloor`))
      (bind _returnvalue (not (`self.HasLandscape` (`PrimitiveComponent.GetOverlappingActors` _array_element null))))
      (bind _returnvalue_2 (not (`self.HasFloor` (`PrimitiveComponent.GetOverlappingActors` _array_element "/Game/EasyBuildingSystem/Blueprints/BuildingObjects/Base/BP_EBS_BuildingObject.BP_EBS_BuildingObject_C"))))
      (if (and _returnvalue _returnvalue_2)
        (set `local.LocalFloorCheck` false :!label _label)
        (return (`local.LocalFloorCheck`)))
      (elif _placedonlandscape
        (if _returnvalue
          (goto _label))
        (elif _returnvalue_2
          (goto _label)))))
  (return (`local.LocalFloorCheck`)))

(fn `CheckSnap`
  (params (TargetObject :type "/Game/EasyBuildingSystem/Blueprints/BuildingObjects/Base/BP_EBS_BuildingObject Object Reference"))
  (returns (Snap :type Boolean))
  (return (`/Game/EasyBuildingSystem/Blueprints/BuildingObjects/Base/BP_EBS_BuildingObject.IsFloor` TargetObject)))

(fn `HasFloor`
  (params (Actors :type "Array of Actor Object Reference"))
  (returns (Result :type Boolean))
  ;[1 1 1] Return true if actors array contains floor.
  (for _array_element Actors
    (bind _asbp_ebs_building_object (cast `/Game/EasyBuildingSystem/Blueprints/BuildingObjects/Base/BP_EBS_BuildingObject` _array_element))
    (if (`/Game/EasyBuildingSystem/Blueprints/BuildingObjects/Base/BP_EBS_BuildingObject.IsFloor` _asbp_ebs_building_object)
      (return true)))
  (return false))

(fn `SetFloorCheckers`)

(fn `SnapToTarget`
  (params (TargetObject :type "/Game/EasyBuildingSystem/Blueprints/BuildingObjects/Base/BP_EBS_BuildingObject Object Reference") (InputRotation :type "Float (double-precision)") (HitLocation :type "Vector Structure") (GridMode :type Boolean) (SnappingMode :type Boolean))
  (returns (NewLocation :type "Vector Structure") (NewRotation :type "Rotator Structure"))
  (locals (LocalZ :type "Float (double-precision)"))
  (bind _x (.x HitLocation))
  (bind _y (.y HitLocation))
  (bind _returnvalue (`KismetMathLibrary.MakeRotator` 0.0 0.0 InputRotation))
  (bind (_gridoffset _gridpropsoffset _gridcorrectoffset) (`self.GetGridOffset` GridMode))
  ;[1 1 1] Get snap location and rotation of Floor Object and Target Unit.
  (if (`/Game/EasyBuildingSystem/Blueprints/BuildingObjects/Base/BP_EBS_BuildingObject.IsFloor` TargetObject)
    (set `local.LocalZ` (`self.GetFloorZ` TargetObject))
    (return (+ (`KismetMathLibrary.MakeVector` (select `bool` GridMode :`false` _x :`true` (+ (* (`KismetMathLibrary.Round` (/ (- _x _gridcorrectoffset) _gridpropsoffset)) _gridpropsoffset) _gridcorrectoffset)) (select `bool` GridMode :`false` _y :`true` (+ (* (`KismetMathLibrary.Round` (/ (- _y _gridcorrectoffset) _gridpropsoffset)) _gridpropsoffset) _gridcorrectoffset)) (`local.LocalZ`)) (`KismetMathLibrary.GreaterGreater_VectorRotator` _gridoffset _returnvalue)) _returnvalue)))

(fn `UserConstructionScript`
  (`parent.UserConstructionScript`)
  (`self.SetFloorCheckers`))