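; Editor utility actor for the Easy Building System that saves, loads, clears and bulk-edits placed building objects.
; Save and load pass every BPI_EBS_SaveActor through a BP_EBS_GameSave slot, respawning objects before restoring their data.
; A box trace sized like MoveCollision gathers building objects, which attach to the actor, detach or get destroyed.
; Copy reuses the save pipeline in memory to spawn duplicates, attaches them and shifts the actor sideways.
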(fn `AddSelectedObjects`
  (bind (_selectcollisionsize_x _selectcollisionsize_y _selectcollisionsize_z) (`KismetMathLibrary.BreakVector` (`self.SelectCollisionSize`)))
  (bind _returnvalue (+ (`self.K2_GetActorLocation`) (`KismetMathLibrary.MakeVector` 0.0 0.0 (* _selectcollisionsize_z -1.0))))
  (bind _outhits (`KismetSystemLibrary.BoxTraceMulti` :`Start` _returnvalue :`End` _returnvalue :`HalfSize` (`KismetMathLibrary.MakeVector` _selectcollisionsize_x _selectcollisionsize_y _selectcollisionsize_z) :`Orientation` (`self.K2_GetActorRotation`) :`TraceChannel` "TraceTypeQuery1" :`DrawDebugType` "ForDuration"))
  (for _array_element _outhits
    (bind _asbp_ebs_building_object (cast `/Game/EasyBuildingSystem/Blueprints/BuildingObjects/Base/BP_EBS_BuildingObject` (`.HitActor` (`GameplayStatics.BreakHitResult` _array_element))))
    (`KismetArrayLibrary.Array_AddUnique` (`self.SelectedObjects`) _asbp_ebs_building_object)))

(fn `AttachSelectedObjects`
  (for _array_element (`self.SelectedObjects`)
    (bind _returnvalue (`self.GetAttachParentActor` _array_element))
    (`/Engine/EditorBlueprintResources/StandardMacros.IsValid` _returnvalue
      (:`Is Valid`
        (`KismetSystemLibrary.PrintString` (`KismetSystemLibrary.GetDisplayName` _returnvalue)))
      (:`Is Not Valid`
        (`self.K2_AttachToActor` _array_element self "None" "KeepWorld" "KeepWorld" "KeepWorld" true)))))

(fn `ClearBuildingObjects`
  (bind _outactors (`GameplayStatics.GetAllActorsWithInterface` "/Game/EasyBuildingSystem/Blueprints/Interfaces/BPI_EBS_SaveActor.BPI_EBS_SaveActor_C"))
  (for _array_element _outactors
    (`self.K2_DestroyActor` _array_element)))

(fn `CopySelectedObjects`
  (locals (LocalCopySave :type "/Game/EasyBuildingSystem/Blueprints/Game/SaveData/BP_EBS_GameSave Object Reference") (LocalCopyActors :type "Array of /Game/EasyBuildingSystem/Blueprints/BuildingObjects/Base/BP_EBS_BuildingObject Object Reference"))
  (bind _localcopysave (`local.LocalCopySave`))
  (bind _savedobjects (`/Game/EasyBuildingSystem/Blueprints/Game/SaveData/BP_EBS_GameSave.SavedObjects` _localcopysave))
  (bind _savedobjects_2 (`/Game/EasyBuildingSystem/Blueprints/Game/SaveData/BP_EBS_GameSave.SavedObjects` (`local.LocalCopySave`)))
  (bind _returnvalue (`BlueprintMapLibrary.Map_Length` _savedobjects_2))
  (`self.DetachSelectedObjects`)
  (bind _returnvalue_2 (`GameplayStatics.CreateSaveGameObject` "/Game/EasyBuildingSystem/Blueprints/Game/SaveData/BP_EBS_GameSave.BP_EBS_GameSave_C"))
  (set `local.LocalCopySave` _returnvalue_2)
  (bind _output_get (set `local.LocalCopyActors` (`self.SelectedObjects`)))
  (for _array_element _output_get
    (message `/Game/EasyBuildingSystem/Blueprints/Interfaces/BPI_EBS_SaveActor.InitSaveID_BPI` _array_element (`local.LocalCopySave`)))
  (for _array_element_2 (`local.LocalCopyActors`)
    (message `/Game/EasyBuildingSystem/Blueprints/Interfaces/BPI_EBS_SaveActor.SaveData_BPI` _array_element_2 (`local.LocalCopySave`)))
  (`KismetArrayLibrary.Array_Clear` (`self.SelectedObjects`))
  (`BlueprintMapLibrary.Map_Clear` _savedobjects)
  (bind _values (`BlueprintMapLibrary.Map_Values` (`/Game/EasyBuildingSystem/Blueprints/Game/SaveData/BP_EBS_GameSave.SavedBuildingObjectsData` _localcopysave)))
  (for _array_element_3 _values
    (bind ((`ID_2_E8B5E8D245D08F40634EDCBFB0A448E9` _id) (`Class_33_7B00E3074E821E574F36EE85E3ED1939` _class) (`Transform_5_F4A8861D41BF0BB9537286A6521E2D6E` _transform)) (break `/Game/EasyBuildingSystem/Blueprints/Game/SaveData/STR_EBS_ObjectData` _array_element_3))
    (bind _returnvalue_3 (`|SpawnActorFromClass` _class _transform "AlwaysSpawn" "OverrideRootScale" null _id true null))
    (`KismetArrayLibrary.Array_Add` (`self.SelectedObjects`) _returnvalue_3)
    (message `/Game/EasyBuildingSystem/Blueprints/Interfaces/BPI_EBS_SaveActor.SetSaveID_BPI` _returnvalue_3 _returnvalue)
    (`BlueprintMapLibrary.Map_Add` _savedobjects_2 _returnvalue _returnvalue_3))
  (bind _values_2 (`BlueprintMapLibrary.Map_Values` _savedobjects))
  (for _array_element_4 _values_2
    (message `/Game/EasyBuildingSystem/Blueprints/Interfaces/BPI_EBS_SaveActor.LoadData_BPI` _array_element_4 (`local.LocalCopySave`)))
  (`self.AttachSelectedObjects`)
  (`self.K2_AddActorWorldOffset` (500.0 0.0 0.0)))

(fn `DestroySelectedObjects`
  (locals (LocalCopySave :type "/Game/EasyBuildingSystem/Blueprints/Game/SaveData/BP_EBS_GameSave Object Reference") (LocalCopyActors :type "Array of /Game/EasyBuildingSystem/Blueprints/BuildingObjects/Base/BP_EBS_BuildingObject Object Reference"))
  (bind _selectedobjects (`self.SelectedObjects`))
  (for _array_element _selectedobjects
    (`self.K2_DestroyActor` _array_element))
  (`KismetArrayLibrary.Array_Clear` _selectedobjects))

(fn `DetachSelectedObjects`
  (for _array_element (`self.SelectedObjects`)
    (`/Game/EasyBuildingSystem/Blueprints/BuildingObjects/Base/BP_EBS_BuildingObject.CreateSocketTransforms` _array_element)
    (if (== (`self.GetAttachParentActor` _array_element) self)
      (`self.K2_DetachFromActor` _array_element "KeepWorld" "KeepWorld" "KeepWorld"))))

(fn `LoadBuildingObjects`
  (locals (LocalGameSave :type "/Game/EasyBuildingSystem/Blueprints/Game/SaveData/BP_EBS_GameSave Object Reference") (LocalSavedActors :type "Array of Actor Object Reference"))
  (bind _savedobjects (`/Game/EasyBuildingSystem/Blueprints/Game/SaveData/BP_EBS_GameSave.SavedObjects` (`local.LocalGameSave`)))
  (bind _returnvalue (`BlueprintMapLibrary.Map_Length` _savedobjects))
  (bind _outactors (`GameplayStatics.GetAllActorsWithInterface` "/Game/EasyBuildingSystem/Blueprints/Interfaces/BPI_EBS_SaveActor.BPI_EBS_SaveActor_C"))
  (for _array_element _outactors
    (`self.K2_DestroyActor` _array_element))
  (bind _returnvalue_2 (`GameplayStatics.LoadGameFromSlot` (`self.SaveSlotName`)))
  (bind _asbp_ebs_game_save (cast `/Game/EasyBuildingSystem/Blueprints/Game/SaveData/BP_EBS_GameSave` _returnvalue_2))
  (bind _output_get (set `local.LocalGameSave` _asbp_ebs_game_save))
  (bind _values (`BlueprintMapLibrary.Map_Values` (`/Game/EasyBuildingSystem/Blueprints/Game/SaveData/BP_EBS_GameSave.SavedBuildingObjectsData` _output_get)))
  (for _array_element_2 _values
    (bind ((`ID_2_E8B5E8D245D08F40634EDCBFB0A448E9` _id) (`Class_33_7B00E3074E821E574F36EE85E3ED1939` _class) (`Transform_5_F4A8861D41BF0BB9537286A6521E2D6E` _transform)) (break `/Game/EasyBuildingSystem/Blueprints/Game/SaveData/STR_EBS_ObjectData` _array_element_2))
    (bind _returnvalue_3 (`|SpawnActorFromClass` _class _transform "AlwaysSpawn" "OverrideRootScale" null _id true null))
    (message `/Game/EasyBuildingSystem/Blueprints/Interfaces/BPI_EBS_SaveActor.SetSaveID_BPI` _returnvalue_3 _returnvalue)
    (`BlueprintMapLibrary.Map_Add` _savedobjects _returnvalue _returnvalue_3))
  (bind _values_2 (`BlueprintMapLibrary.Map_Values` (`/Game/EasyBuildingSystem/Blueprints/Game/SaveData/BP_EBS_GameSave.SavedObjects` _output_get)))
  (for _array_element_3 _values_2
    (message `/Game/EasyBuildingSystem/Blueprints/Interfaces/BPI_EBS_SaveActor.LoadData_BPI` _array_element_3 (`local.LocalGameSave`)))
  (`KismetSystemLibrary.PrintString` "Game Loaded!" true true (struct :`R` 1.0 :`G` 0.041493 :`A` 1.0) 10.0))

(fn `SaveBuildingObjects`
  (locals (LocalGameSave :type "/Game/EasyBuildingSystem/Blueprints/Game/SaveData/BP_EBS_GameSave Object Reference") (LocalSavedActors :type "Array of Actor Object Reference"))
  (bind _returnvalue (`GameplayStatics.CreateSaveGameObject` "/Game/EasyBuildingSystem/Blueprints/Game/SaveData/BP_EBS_GameSave.BP_EBS_GameSave_C"))
  (set `local.LocalGameSave` _returnvalue)
  (bind _outactors (`GameplayStatics.GetAllActorsWithInterface` "/Game/EasyBuildingSystem/Blueprints/Interfaces/BPI_EBS_SaveActor.BPI_EBS_SaveActor_C"))
  (bind _output_get (set `local.LocalSavedActors` _outactors))
  (for _array_element _output_get
    (message `/Game/EasyBuildingSystem/Blueprints/Interfaces/BPI_EBS_SaveActor.InitSaveID_BPI` _array_element (`local.LocalGameSave`)))
  (for _array_element_2 (`local.LocalSavedActors`)
    (message `/Game/EasyBuildingSystem/Blueprints/Interfaces/BPI_EBS_SaveActor.SaveData_BPI` _array_element_2 (`local.LocalGameSave`)))
  (bind _returnvalue_2 (`GameplayStatics.SaveGameToSlot` (`local.LocalGameSave`) (`self.SaveSlotName`)))
  (if _returnvalue_2
    (`KismetSystemLibrary.PrintString` "Game Saved!" true true (struct :`R` 1.0 :`A` 1.0) 10.0)
    (else
      (`KismetSystemLibrary.PrintString` "Game dont Saved!!!" true true (struct :`R` 1.0 :`G` 0.036246 :`A` 1.0) 10.0))))

(fn `UserConstructionScript`
  (bind _selectcollisionsize (`self.SelectCollisionSize`))
  (bind _movecollision (`self.MoveCollision`))
  (`SceneComponent.K2_SetRelativeLocation` _movecollision (`KismetMathLibrary.MakeVector` 0.0 0.0 (* (.z _selectcollisionsize) -1.0)) false false)
  (`BoxComponent.SetBoxExtent` _movecollision _selectcollisionsize true))