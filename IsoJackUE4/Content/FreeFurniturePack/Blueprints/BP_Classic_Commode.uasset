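; Classic commode furniture actor whose five drawers slide out when the ThirdPersonCharacter enters its Box trigger and slide back when it leaves.
; Two cross-reset DoOnce gates let begin and end overlap each fire their move once, alternating open and close.
; Five identical Open Drawer subgraphs use MoveComponentTo to offset each drawer along relative Y over a fixed time.
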(event `self.Box.OnComponentBeginOverlap`
  (params (OverlappedComponent :type "PrimitiveComponent Object Reference") (OtherActor :type "Actor Object Reference") (OtherComp :type "PrimitiveComponent Object Reference") (OtherBodyIndex :type Integer) (bFromSweep :type Boolean) (SweepResult :type "HitResult Structure (by ref)"))
  (bind _sm_classic_commode_drawer_1_1 (`self.SM_Classic_Commode_Drawer_1_1`))
  (bind _sm_classic_commode_drawer_2 (`self.SM_Classic_Commode_Drawer_2`))
  (bind _sm_classic_commode_drawer_1_2 (`self.SM_Classic_Commode_Drawer_1_2`))
  (bind _sm_classic_commode_drawer_2_1 (`self.SM_Classic_Commode_Drawer_2_1`))
  (bind _sm_classic_commode_drawer_1 (`self.SM_Classic_Commode_Drawer_1`))
  (bind _relativelocation (`SceneComponent.RelativeLocation` _sm_classic_commode_drawer_1_1))
  (bind _relativelocation_2 (`SceneComponent.RelativeLocation` _sm_classic_commode_drawer_2))
  (bind _relativelocation_3 (`SceneComponent.RelativeLocation` _sm_classic_commode_drawer_1_2))
  (bind _relativelocation_4 (`SceneComponent.RelativeLocation` _sm_classic_commode_drawer_2_1))
  (bind _relativelocation_5 (`SceneComponent.RelativeLocation` _sm_classic_commode_drawer_1))
  (cast `/Game/ThirdPersonBP/Blueprints/ThirdPersonCharacter` OtherActor)
  (`|ExecutionSequence`
    (:`then_0`
      (`/Engine/EditorBlueprintResources/StandardMacros.DoOnce` false :!label _label
        (:`Completed`
          (`|ExecutionSequence`
            (:`then_0`
              (`KismetSystemLibrary.MoveComponentTo` _sm_classic_commode_drawer_1_1 (+ _relativelocation (0.0 30.0 0.0)) (struct) false false 2.0))
            (:`then_1`
              (`KismetSystemLibrary.MoveComponentTo` _sm_classic_commode_drawer_2 (+ _relativelocation_2 (0.0 30.0 0.0)) (struct) false false 2.0))
            (:`then_2`
              (`KismetSystemLibrary.MoveComponentTo` _sm_classic_commode_drawer_1_2 (+ _relativelocation_3 (0.0 30.0 0.0)) (struct) false false 2.0))
            (:`then_3`
              (`KismetSystemLibrary.MoveComponentTo` _sm_classic_commode_drawer_2_1 (+ _relativelocation_4 (0.0 30.0 0.0)) (struct) false false 2.0))
            (:`then_4`
              (`KismetSystemLibrary.MoveComponentTo` _sm_classic_commode_drawer_1 (+ _relativelocation_5 (0.0 30.0 0.0)) (struct) false false 2.0))))))
    (:`then_1`
      (goto _label_2 :!via `Reset`))))

(event `self.Box.OnComponentEndOverlap`
  (params (OverlappedComponent :type "PrimitiveComponent Object Reference") (OtherActor :type "Actor Object Reference") (OtherComp :type "PrimitiveComponent Object Reference") (OtherBodyIndex :type Integer))
  (bind _sm_classic_commode_drawer_1_1 (`self.SM_Classic_Commode_Drawer_1_1`))
  (bind _sm_classic_commode_drawer_2 (`self.SM_Classic_Commode_Drawer_2`))
  (bind _sm_classic_commode_drawer_1_2 (`self.SM_Classic_Commode_Drawer_1_2`))
  (bind _sm_classic_commode_drawer_2_1 (`self.SM_Classic_Commode_Drawer_2_1`))
  (bind _sm_classic_commode_drawer_1 (`self.SM_Classic_Commode_Drawer_1`))
  (cast `/Game/ThirdPersonBP/Blueprints/ThirdPersonCharacter` OtherActor)
  (`|ExecutionSequence`
    (:`then_0`
      (goto _label :!via `Reset`))
    (:`then_1`
      (`/Engine/EditorBlueprintResources/StandardMacros.DoOnce` false :!label _label_2
        (:`Completed`
          (`|ExecutionSequence`
            (:`then_0`
              (`KismetSystemLibrary.MoveComponentTo` _sm_classic_commode_drawer_1_1 (+ (`SceneComponent.RelativeLocation` _sm_classic_commode_drawer_1_1) (0.0 -30.0 0.0)) (struct) false false 2.0))
            (:`then_1`
              (`KismetSystemLibrary.MoveComponentTo` _sm_classic_commode_drawer_2 (+ (`SceneComponent.RelativeLocation` _sm_classic_commode_drawer_2) (0.0 -30.0 0.0)) (struct) false false 2.0))
            (:`then_2`
              (`KismetSystemLibrary.MoveComponentTo` _sm_classic_commode_drawer_1_2 (+ (`SceneComponent.RelativeLocation` _sm_classic_commode_drawer_1_2) (0.0 -30.0 0.0)) (struct) false false 2.0))
            (:`then_3`
              (`KismetSystemLibrary.MoveComponentTo` _sm_classic_commode_drawer_2_1 (+ (`SceneComponent.RelativeLocation` _sm_classic_commode_drawer_2_1) (0.0 -30.0 0.0)) (struct) false false 2.0))
            (:`then_4`
              (`KismetSystemLibrary.MoveComponentTo` _sm_classic_commode_drawer_1 (+ (`SceneComponent.RelativeLocation` _sm_classic_commode_drawer_1) (0.0 -30.0 0.0)) (struct) false false 2.0))))))))

(fn `UserConstructionScript`)